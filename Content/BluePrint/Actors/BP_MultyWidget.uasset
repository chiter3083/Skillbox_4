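; BP_MultyWidget is an actor with a Widget component showing an electric panel UI for a configurable list of actors.
; On BeginPlay it casts the component's user widget to UMG_ElectricPanel and caches the reference.
; It then loops over ActorsToInteract and has the panel construct a new line for each entry, passing its name and actor reference.
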(event EventBeginPlay
  (|CallParentFunction)
  (bind _asumg_electric_panel (Utilities|Casting|CastToUMG_ElectricPanel (UserInterface|GetUserWidgetObject (Variables|Default|GetWidget))))
  (Variables|Default|SetUMG%20Electric%20Panel _asumg_electric_panel)
  (for _array_element (Variables|Default|GetActorsToInteract)
    (Default|ConstructNewLine (Variables|Default|GetUMG%20Electric%20Panel) (.ActorName (Utilities|Struct|BreakStruct_ActorsToInteract _array_element)) (.Actor (Utilities|Struct|BreakStruct_ActorsToInteract _array_element)))))

(event Collision|EventActorBeginOverlap
  (params (OtherActor :type Actor%20Object%20Reference))
  (|CallParentFunction OtherActor) ; This node is disabled and will not be called.\nDrag off pins to build functionality.
)

(event EventTick
  (params (DeltaSeconds :type Float%20%28single-precision%29))
  (|CallParentFunction DeltaSeconds) ; This node is disabled and will not be called.\nDrag off pins to build functionality.
)

(fn ConstructionScript
  (|CallParentFunction))