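; BP_MeshShowcase is a display actor that shows a configurable static mesh with an attached commentary box.
; The construction script applies the mesh and passes its text lines to the child BP_Commentary_Box, cached as a reference.
; Trace interaction toggles a gate that spins the mesh around yaw each tick.
; Look-at and look-away events turn the commentary on and off.
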(event Custom|ToggleInfo)

(event EventBeginPlay)

(event Collision|EventActorBeginOverlap
  (params (OtherActor :type Actor%20Object%20Reference)))

(event EventTick
  (params (DeltaSeconds :type Float%20%28single-precision%29))
  (Utilities|FlowControl|Gate true
    (:Exit
      (Transformation|AddLocalRotation (Variables|Default|GetStaticMesh) "0.000000,1.000000,0.000000" false false))))

(event EventInteractbyTrace
  (params (OutHit :type Hit%20Result%20Structure))
  (Utilities|FlowControl|Gate true) ; enters at Toggle
)

(event EventLookAway
  (Default|TurnOff (Variables|Default|GetTipActorReference)))

(event EventLookat
  (Default|Turnon (Variables|Default|GetTipActorReference)))

(fn ConstructionScript
  (Components|StaticMesh|SetStaticMesh (Variables|Default|GetStaticMesh) (Variables|Default|GetMesh))
  (bind _asbp_commentary_box (Utilities|Casting|CastToBP_Commentary_Box (Variables|/Script/Engine.ChildActorComponent|GetChildActor (Variables|Default|GetBP_Commentary_Box))))
  (bind _output_get (Variables|Default|SetTipActorReference _asbp_commentary_box))
  (Variables|/Game/Assets/Blueprints/BP_Commentary_Box.BP_Commentary_Box_C|SetLines _output_get (Variables|Default|GetLines)))