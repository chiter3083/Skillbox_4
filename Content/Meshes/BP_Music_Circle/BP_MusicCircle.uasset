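; Music circle actor running a Simon-style memory game with tagged button meshes, colour swaps and sounds.
; A looping timer plays a random note sequence, faster as it lengthens, then opens input through InteractbyTrace.
; Completing a sequence generates a fresh one a note longer, while a wrong button resets to one note.
; The SM2M mesh toggles Play/Stop, gating button presses but not playback.
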(event Custom|PushButton
  (params (ActorComponent :type Actor%20Component%20Object%20Reference)))

(event EventBeginPlay
  (Variables|Default|SetCurrentSequenceLoop 0)
  (CallFunction|CalculateNotes)
  (CallFunction|PlayNoteSequence))

(event Collision|EventActorBeginOverlap
  (params (OtherActor :type Actor%20Object%20Reference)))

(event EventTick
  (params (DeltaSeconds :type Float%20%28single-precision%29)))

(event EventInteractbyTrace
  (params (OutHit :type Hit%20Result%20Structure))
  (if (Variables|Default|GetisInputMode?)
    (bind (_succes _correct _buttoncomponent _buttonid) (CallFunction|TryPressButton (.HitComponent (Collision|BreakHitResult OutHit))))
    (if _succes
      (CallFunction|InteractButton _correct _buttonid))))

(fn ConstructionScript
  (CallFunction|UpdateBaseColors)
  (CallFunction|CollectButtons))

(fn UpdateBaseColors
  (Rendering|Material|SetMaterial (Variables|Default|GetBasa) 0 "/Game/Material/MusicCircle/MI_ColorBlue.MI_ColorBlue"))

(fn CollectButtons
  (Utilities|Array|Clear (Variables|Default|GetButtons))
  (Variables|Default|SetButtons (Actor|GetComponentsbyTag "/Script/Engine.ActorComponent" "MusicButton"))
  (Variables|Default|SetButtonsCount (Utilities|Array|Length (Variables|Default|GetButtons))))

(fn CalculateNotes
  (Utilities|Array|Clear (Variables|Default|GetNotes))
  (LocalVariables|SetLocalMaxNotes (Variables|Default|GetCurrentSequenceLoop))
  (for _index (range 0 (LocalVariables|GetLocalMaxNotes))
    (Utilities|Array|Add (Variables|Default|GetNotes) (Math|Random|RandomInteger (Variables|Default|GetButtonsCount))))
  (Variables|Default|SetSizeOfSequence (Utilities|Array|Length (Variables|Default|GetNotes))))

(fn PlayNoteSequence
  (Variables|Default|SetisInputMode? false)
  (Variables|Default|SetNoteLoop 0)
  (bind _returnvalue (Utilities|Time|SetTimerbyFunctionName 0 "PlayNote" (/ (Variables|Default|GetSpeed) (Variables|Default|GetSizeOfSequence)) true))
  (Variables|Default|SetPlayNoteTimerHandle _returnvalue)
  (Rendering|Components|TextRender|SetText (Variables|Default|GetTextLevel) (Utilities|Text|ToText(Integer) (Variables|Default|GetSizeOfSequence))))

(fn PlayNote
  (if (< (Variables|Default|GetNoteLoop) (Variables|Default|GetSizeOfSequence))
    (Variables|Default|SetCurrentNote (Utilities|Array|Get(acopy) (Variables|Default|GetNotes) (Variables|Default|GetNoteLoop)))
    (if (Variables|Default|GetisTurnOn?)
      (Variables|Default|SetisTurnOn? false)
      (bind _asstatic_mesh_component (Utilities|Casting|CastToStaticMeshComponent (Utilities|Array|Get(acopy) (Variables|Default|GetButtons) (Variables|Default|GetCurrentNote))))
      (Rendering|Material|SetMaterial _asstatic_mesh_component 0 "/Game/Material/MusicCircle/MI_ColorGreen.MI_ColorGreen")
      (Audio|PlaySoundatLocation (Utilities|Array|Get(acopy) (Variables|Default|GetSounds) (Variables|Default|GetCurrentNote)) (Transformation|GetWorldLocation (Variables|Default|GetBasa)) "0, 0, 0" 1.0 1.0 0.0 0 0 0 0)
      (else
        (Variables|Default|SetisTurnOn? true)
        (bind _asstatic_mesh_component_2 (Utilities|Casting|CastToStaticMeshComponent (Utilities|Array|Get(acopy) (Variables|Default|GetButtons) (Variables|Default|GetCurrentNote))))
        (Rendering|Material|SetMaterial _asstatic_mesh_component_2 0 "/Game/Material/MusicCircle/MI_ColorGray.MI_ColorGray")
        (Math|Integer|IncrementInt (Variables|Default|GetNoteLoop))))
    (else
      (Utilities|Time|ClearandInvalidateTimerbyHandle (Variables|Default|GetPlayNoteTimerHandle))
      (Variables|Default|SetisInputMode? true)
      (Variables|Default|SetNoteLoop 0))))

(fn UpdateGameLoop
  (Math|Integer|IncrementInt (Variables|Default|GetCurrentSequenceLoop)
    (:%20%20
      (CallFunction|CalculateNotes)
      (CallFunction|PlayNoteSequence))))

(fn TryPressButton
  (params (Object :type Actor%20Component%20Object%20Reference))
  (bind _asstatic_mesh_component (Utilities|Casting|CastToStaticMeshComponent Object)
    (:then
      (bind _isplay_ (CallFunction|StopPlay _asstatic_mesh_component))
      (if _isplay_
        (bind _output_get (LocalVariables|SetLocalButton _asstatic_mesh_component))
        (LocalVariables|SetLocalButtonID (Utilities|Array|FindItem (Variables|Default|GetButtons) _output_get))
        (if (> (Utilities|Array|FindItem (Variables|Default|GetButtons) _output_get) -1)
          (if (== (Utilities|Array|FindItem (Variables|Default|GetButtons) _output_get) (Utilities|Array|Get(acopy) (Variables|Default|GetNotes) (Variables|Default|GetNoteLoop)))
            (Rendering|Material|SetMaterial (LocalVariables|GetLocalButton) 0 "/Game/Material/MusicCircle/MI_ColorGreen.MI_ColorGreen")
            (Math|Integer|IncrementInt (Variables|Default|GetNoteLoop)
              (:%20%20
                (if (>= (Variables|Default|GetNoteLoop) (Variables|Default|GetSizeOfSequence))
                  (CallFunction|UpdateGameLoop))
                (return true true (LocalVariables|GetLocalButton) (LocalVariables|GetLocalButtonID))))
            (else
              (Rendering|Material|SetMaterial (LocalVariables|GetLocalButton) 0 "/Game/Material/MusicCircle/MI_ColorRed.MI_ColorRed")
              (Rendering|Material|SetMaterial (Variables|Default|GetSM_2_M) 0 "/Game/Material/MusicCircle/M_ColorBase.M_ColorBase")
              (Variables|Default|SetCurrentSequenceLoop 0)
              (CallFunction|UpdateGameLoop)
              (return true false (LocalVariables|GetLocalButton) (LocalVariables|GetLocalButtonID)))))))
    (:CastFailed
      (return true false 0 0))))

(fn InteractButton
  (params (Correct :type Boolean) (ButtonID :type Integer))
  (Variables|Default|SetActiveButton ButtonID)
  (Utilities|Time|SetTimerbyFunctionName 0 "ClearActiveButton" (/ (Variables|Default|GetSpeed) 2.0))
  (Audio|PlaySoundatLocation (Utilities|Array|Get(acopy) (Variables|Default|GetSounds) (Variables|Default|GetActiveButton)) (Transformation|GetWorldLocation (Variables|Default|GetBasa)) "0, 0, 0" 1.0 1.0 0.0 0 0 0 0))

(fn ClearActiveButton
  (bind _asstatic_mesh_component (Utilities|Casting|CastToStaticMeshComponent (Utilities|Array|Get(acopy) (Variables|Default|GetButtons) (Variables|Default|GetActiveButton))))
  (Rendering|Material|SetMaterial _asstatic_mesh_component 0 "/Game/Material/MusicCircle/MI_ColorGray.MI_ColorGray"))

(fn StopPlay
  (params (Button :type Static%20Mesh%20Component%20Object%20Reference))
  (if (== Button (Variables|Default|GetSM_2_M))
    (Rendering|Components|TextRender|SetText (Variables|Default|GetTextBool) (Utilities|String|SelectText "Stop" "Play" (Variables|Default|GetisPlay?)))
    (if (Variables|Default|GetisPlay?)
      (bind _output_get (Variables|Default|SetisPlay? false))
      (Rendering|Material|SetMaterial (Variables|Default|GetSM_2_M) 0 "/Game/Material/MusicCircle/MI_ColorYellow.MI_ColorYellow")
      (return _output_get)
      (else
        (bind _output_get_2 (Variables|Default|SetisPlay? true))
        (Rendering|Material|SetMaterial (Variables|Default|GetSM_2_M) 0 "/Game/Material/MusicCircle/M_ColorBase.M_ColorBase")
        (return _output_get_2)))
    (else
      (return (Variables|Default|GetisPlay?)))))